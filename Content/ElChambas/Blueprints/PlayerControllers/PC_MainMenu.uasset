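; Player controller for the main menu that manages the main menu and settings widgets.
; After a short delay on BeginPlay it shows the main menu and switches input to UI only.
; A ShowHideWidget event routes to functions that switch on a widget enum, lazily creating and caching each widget before adding or removing it from the viewport.
; A getter returns the controller itself, likely as an interface implementation.
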(event Custom|ShowHideWidget
  (params (Show :type Boolean) (Widget :type E_WidgetsMainMenu%20Enum :default "NewEnumerator0"))
  (if Show
    (CallFunction|FShowWidget Widget)
    (else
      (CallFunction|FHideWidget Widget))))

(event EventBeginPlay
  (Utilities|FlowControl|Delay 3.5)
  (CallFunction|ShowHideWidget true "NewEnumerator0")
  (Input|SetInputModeUIOnly self 0 "DoNotLock" false))

(fn ConstructionScript)

(fn FShowWidget
  (params (Widget :type E_WidgetsMainMenu%20Enum :default "NewEnumerator0"))
  (switch Utilities|FlowControl|Switch|SwitchonE_WidgetsMainMenu Widget
    (:NewEnumerator0
      (Variables|Default|GetWB_MainMenu
        (:then
          _)
        (:else
          (bind _returnvalue (UserInterface|CreateWidget "/Game/ElChambas/UI/Widgets/WB_MainMenu.WB_MainMenu_C"))
          (bind _output_get (Variables|Default|SetWB_MainMenu _returnvalue))))
      (UserInterface|Viewport|AddtoViewport _output_get 0))
    (:NewEnumerator1
      (Variables|Default|GetWB_Settings
        (:then
          _)
        (:else
          (bind _returnvalue_2 (UserInterface|CreateWidget "/Game/ElChambas/UI/Widgets/WB_Settings.WB_Settings_C"))
          (bind _output_get_2 (Variables|Default|SetWB_Settings _returnvalue_2))))
      (UserInterface|Viewport|AddtoViewport _output_get_2 0))))

(fn FHideWidget
  (params (Widget :type E_WidgetsMainMenu%20Enum :default "NewEnumerator0"))
  (switch Utilities|FlowControl|Switch|SwitchonE_WidgetsMainMenu Widget
    (:NewEnumerator0
      (bind _wb_mainmenu (Variables|Default|GetWB_MainMenu)
        (:then
          (Widget|RemovefromParent _wb_mainmenu))
        (:else)))
    (:NewEnumerator1
      (bind _wb_settings (Variables|Default|GetWB_Settings)
        (:then
          (Widget|RemovefromParent _wb_settings))
        (:else)))))

(fn GetPCMainMenu
  (return self))
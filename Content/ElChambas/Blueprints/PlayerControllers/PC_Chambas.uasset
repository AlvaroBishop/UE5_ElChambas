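; PC_Chambas is a player controller that manages UI widgets for El Chambas, showing the Camionero widget when play begins.
; On BeginPlay it sets input to UI only and calls the ShowHideWidget event, which routes to show or hide functions by a boolean.
; Those functions switch on a widget enum, lazily creating and caching the Camionero widget before adding it to the viewport, or removing it from parent if valid.
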(event Custom|ShowHideWidget
  (params (Show :type Boolean) (Widget :type E_Widgets%20Enum :default "NewEnumerator0"))
  (if Show
    (CallFunction|FShowWidget Widget)
    (else
      (CallFunction|FHideWidget Widget))))

(event EventBeginPlay
  (Input|SetInputModeUIOnly self 0 "DoNotLock" false)
  (CallFunction|ShowHideWidget true "NewEnumerator1"))

(fn ConstructionScript)

(fn FShowWidget
  (params (Widget :type E_Widgets%20Enum :default "NewEnumerator0"))
  (switch Utilities|FlowControl|Switch|SwitchonE_Widgets Widget
    (:NewEnumerator1
      (Variables|Default|GetWB_Camionero
        (:then
          _)
        (:else
          (bind _returnvalue (UserInterface|CreateWidget "/Game/ElChambas/UI/Widgets/WB_Camionero.WB_Camionero_C"))
          (bind _output_get (Variables|Default|SetWB_Camionero _returnvalue))))
      (UserInterface|Viewport|AddtoViewport _output_get 0))))

(fn FHideWidget
  (params (Widget :type E_Widgets%20Enum :default "NewEnumerator0"))
  (switch Utilities|FlowControl|Switch|SwitchonE_Widgets Widget
    (:NewEnumerator1
      (bind _wb_camionero (Variables|Default|GetWB_Camionero)
        (:then
          (Widget|RemovefromParent _wb_camionero))
        (:else)))))
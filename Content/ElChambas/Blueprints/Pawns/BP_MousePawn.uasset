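; BP_MousePawn is a pawn that lets the player drag Movable components with the mouse, with Space toggling grab mode and the cursor.
; Left click traces under the cursor and stores the hit component, distance and grab offset until release.
; Tick projects the mouse ray to that distance, pulling simulating bodies via a PhysicsHandle with a debug line.
; Non-simulating components are repositioned directly, preserving the grab offset.
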(event EventTick
  (params (DeltaSeconds :type Float%20%28single-precision%29))
  (bind _originaldistancetoobject (Variables|Default|GetOriginalDistanceToObject))
  (bind _mouselocation (CallFunction|FGetMouseLocation _originaldistancetoobject))
  (if (Variables|Default|GetbIsGrabMode)
    (bind _grabbedcomponent (Variables|Default|GetGrabbedComponent)
      (:then
        (if (Physics|IsSimulatingPhysics _grabbedcomponent "None")
          (Physics|Components|PhysicsHandle|SetTargetLocation (Variables|Default|GetPhysicsHandle) _mouselocation)
          (Rendering|Debug|DrawDebugLine :LineStart _mouselocation :LineEnd (Math|Transform|TransformLocation (Transformation|GetWorldTransform (Variables|Default|GetGrabbedComponent)) (Variables|Default|GetRelativeGrabLocation)) :Thickness 15.0)
          (else
            (Transformation|SetWorldLocation (Variables|Default|GetGrabbedComponent) (Math|Transform|InverseTransformLocation (Math|Conversions|ToTransform(Vector) (Variables|Default|GetRelativeGrabLocation)) (CallFunction|FGetMouseLocation (Variables|Default|GetOriginalDistanceToObject))) false false))))
      (:else))))

(event Input|MouseEvents|LeftMouseButton
  (params (Key :type Key%20Structure))
  (bind _returnvalue (Game|GetPlayerController 0))
  (bind _bisgrabmode (Variables|Default|GetbIsGrabMode))
  (bind _hitresult (Game|Player|GetHitResultUnderCursorbyChannel _returnvalue "TraceTypeQuery1" true))
  (bind (_bblockinghit _binitialoverlap _time _distance _location _impactpoint _normal _impactnormal _physmat _hitactor _hitcomponent) (Collision|BreakHitResult _hitresult))
  (bind (_bblockinghit_2 _binitialoverlap_2 _time_2 _distance_2 _location_2 _impactpoint_2 _normal_2 _impactnormal_2 _physmat_2 _hitactor_2 _hitcomponent_2) (Collision|BreakHitResult _hitresult))
  (:Pressed
    (if _bisgrabmode
      (Utilities|IsValid _hitcomponent_2
        (:Is%20Valid
          (Transformation|SetMobility _hitcomponent_2 "Movable")
          (Physics|SetSimulatePhysics _hitcomponent_2 true)
          (Physics|SetEnableGravity _hitcomponent_2 false)
          (if (and (Utilities|Enum|Equal(Enum) (Variables|/Script/Engine.SceneComponent|GetMobility _hitcomponent_2) "Movable") _bblockinghit_2)
            (Variables|Default|SetOriginalDistanceToObject _distance_2)
            (bind _output_get (Variables|Default|SetGrabbedComponent _hitcomponent_2))
            (if (Physics|IsSimulatingPhysics _output_get "None")
              (Class|PhysicsHandleComponent|GrabComponentatLocation (Variables|Default|GetPhysicsHandle) (Variables|Default|GetGrabbedComponent) "None" _location)
              (Variables|Default|SetRelativeGrabLocation (Math|Transform|InverseTransformLocation (Transformation|GetWorldTransform (Variables|Default|GetGrabbedComponent)) _location))
              (else
                (Variables|Default|SetRelativeGrabLocation (Math|Transform|InverseTransformLocation (Math|Conversions|ToTransform(Vector) (Transformation|GetWorldLocation _hitcomponent)) _location)))))))))
  (:Released
    (if _bisgrabmode
      (Transformation|SetMobility (Variables|Default|GetGrabbedComponent) "Static")
      (Physics|SetSimulatePhysics (Variables|Default|GetGrabbedComponent) false)
      (Variables|Default|SetGrabbedComponent 0)
      (Physics|Components|PhysicsHandle|ReleaseComponent (Variables|Default|GetPhysicsHandle)))))

(event Input|KeyboardEvents|SpaceBar
  (params (Key :type Key%20Structure))
  (bind _returnvalue (Game|GetPlayerController 0))
  (:Pressed
    (Variables|/Script/Engine.PlayerController|SetbShowMouseCursor _returnvalue (not (Variables|/Script/Engine.PlayerController|GetbShowMouseCursor _returnvalue)))
    (Variables|Default|SetbIsGrabMode (not (Variables|Default|GetbIsGrabMode)))))

(fn ConstructionScript)

(fn FGetMouseLocation
  (params (Original%20Distance%20To%20Object :type Float%20%28double-precision%29))
  (bind _returnvalue (Game|GetPlayerController 0))
  (bind (_worldlocation _worlddirection) (Game|Player|ConvertMouseLocationToWorldSpace _returnvalue))
  (return (+ _worldlocation (* _worlddirection Original%20Distance%20To%20Object))))
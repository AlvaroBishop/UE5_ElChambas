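; Player character for the Camionero minigame, a quick-time balance challenge driven by timed prompts on the WBCamionero widget.
; A looping timer randomly fires a bottle to jump, a left or right fall, or a braking grab.
; Timelines roll the actor or change spring arm length, and matching move events reverse the tilt or flag the grab.
; Missed tilts and grabs only print "Perdiste"; the bottle has no fail check here.
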(event Custom|MoveDown
  (bind _player_controller (Variables|Default|GetPlayer%20Controller))
  (bind _wb_camionero (Variables|/Game/ElChambas/Blueprints/PlayerControllers/PC_Chambas.PC_Chambas_C|GetWB_Camionero _player_controller))
  (if (Variables|Default|GetIsDownEvent)
    (Variables|Default|SetbSeAgarro true)
    (Default|ShowHideKey _wb_camionero false (Variables|/Game/ElChambas/UI/Widgets/WB_Camionero.WB_Camionero_C|GetDown _wb_camionero))
    (Default|SetWarningText _wb_camionero "" false)))

(event Custom|MoveUp
  (bind _player_controller (Variables|Default|GetPlayer%20Controller))
  (bind _wb_camionero (Variables|/Game/ElChambas/Blueprints/PlayerControllers/PC_Chambas.PC_Chambas_C|GetWB_Camionero _player_controller))
  (Character|Jump)
  (Default|ShowHideKey _wb_camionero false (Variables|/Game/ElChambas/UI/Widgets/WB_Camionero.WB_Camionero_C|GetUp _wb_camionero))
  (Default|SetWarningText (Variables|/Game/ElChambas/Blueprints/PlayerControllers/PC_Chambas.PC_Chambas_C|GetWB_Camionero (Variables|Default|GetPlayer%20Controller)) "" false))

(event Custom|UpEvent
  (bind _player_controller (Variables|Default|GetPlayer%20Controller))
  (bind _player_controller_2 (Variables|Default|GetPlayer%20Controller))
  (bind _wb_camionero (Variables|/Game/ElChambas/Blueprints/PlayerControllers/PC_Chambas.PC_Chambas_C|GetWB_Camionero _player_controller))
  (bind _wb_camionero_2 (Variables|/Game/ElChambas/Blueprints/PlayerControllers/PC_Chambas.PC_Chambas_C|GetWB_Camionero _player_controller_2))
  (bind _returnvalue (Game|SpawnActorfromClass "/Game/ElChambas/Blueprints/Actors/Camionero/BP_Bottle.BP_Bottle_C" (Math|Transform|MakeTransform "932.705184,-29.768055,158.924578" "0.000000,0.000000,-90.000000" "1.000000,1.000000,1.000000") "AlwaysSpawn" "MultiplyWithRoot" 0 0))
  (Utilities|FlowControl|Delay 2.0)
  (Default|ShowHideKey _wb_camionero true (Variables|/Game/ElChambas/UI/Widgets/WB_Camionero.WB_Camionero_C|GetUp _wb_camionero))
  (Default|SetWarningText _wb_camionero "Aguas!" true)
  (Utilities|FlowControl|Sequence
    (:then_0
      (Actor|SetLifeSpan _returnvalue 2.0))
    (:then_1
      (Utilities|FlowControl|Delay 2.0)
      (Default|ShowHideKey _wb_camionero_2 false (Variables|/Game/ElChambas/UI/Widgets/WB_Camionero.WB_Camionero_C|GetUp _wb_camionero_2))
      (Default|SetWarningText _wb_camionero_2 "" false))))

(event Custom|Reverse
  (bind _player_controller (Variables|Default|GetPlayer%20Controller))
  (bind _wb_camionero (Variables|/Game/ElChambas/Blueprints/PlayerControllers/PC_Chambas.PC_Chambas_C|GetWB_Camionero _player_controller))
  (Variables|Default|SetIsDownEvent false)
  (Default|ShowHideKey _wb_camionero false (Variables|/Game/ElChambas/UI/Widgets/WB_Camionero.WB_Camionero_C|GetDown _wb_camionero))
  (bind _alpha (Timeline|FrenaEvent Reverse)
    (:Update
      (Variables|/Script/Engine.SpringArmComponent|SetTargetArmLength (Variables|Default|GetSpringArm) (Math|Float|Lerp (Variables|Default|GetStart%20Target%20Arm%20Length) 3e+02 _alpha)))
    (:Finished
      (if (Variables|Default|GetIsDownEvent)
        (if (Variables|Default|GetbSeAgarro)
          (CallFunction|Reverse)
          (else
            (Development|PrintString "Perdiste")))
        (else
          (CallFunction|ResetDownEvent))))))

(event Custom|ResetDownEvent
  (bind _player_controller (Variables|Default|GetPlayer%20Controller))
  (bind _wb_camionero (Variables|/Game/ElChambas/Blueprints/PlayerControllers/PC_Chambas.PC_Chambas_C|GetWB_Camionero _player_controller))
  (Utilities|FlowControl|DoOnce false) ; enters at Reset
)

(event Custom|ClearHandles
  (Utilities|Time|ClearandInvalidateTimerbyHandle (Variables|Default|GetGameManagerTimerHandle)))

(event Custom|StopMoveRight
  (bind _returnvalue (Transformation|GetActorRotation))
  (bind _player_controller (Variables|Default|GetPlayer%20Controller))
  (bind _wb_camionero (Variables|/Game/ElChambas/Blueprints/PlayerControllers/PC_Chambas.PC_Chambas_C|GetWB_Camionero _player_controller))
  (Default|ShowHideKey _wb_camionero false (Variables|/Game/ElChambas/UI/Widgets/WB_Camionero.WB_Camionero_C|GetRight _wb_camionero))
  (Default|SetWarningText _wb_camionero "Te !" false)
  (bind _alpha (Timeline|Timeline Reverse)
    (:Update
      (Transformation|SetActorRelativeRotation (Math|Rotator|MakeRotator (Math|Float|Lerp 0.0 35.0 _alpha) (.pitch _returnvalue) (.yaw _returnvalue))))
    (:Finished
      (if (not (== (Math|Float|Lerp 0.0 35.0 _alpha) 0.0))
        (Development|PrintString "Perdiste")))))

(event Custom|MoveRight
  (CallFunction|StopMoveRight))

(event Custom|StopMoveLeft
  (bind _returnvalue (Transformation|GetActorRotation))
  (bind _player_controller (Variables|Default|GetPlayer%20Controller))
  (bind _wb_camionero (Variables|/Game/ElChambas/Blueprints/PlayerControllers/PC_Chambas.PC_Chambas_C|GetWB_Camionero _player_controller))
  (Default|ShowHideKey _wb_camionero false (Variables|/Game/ElChambas/UI/Widgets/WB_Camionero.WB_Camionero_C|GetLeft _wb_camionero))
  (Default|SetWarningText _wb_camionero "" false)
  (bind _alpha (Timeline|Timeline_1 Reverse)
    (:Update
      (Transformation|SetActorRelativeRotation (Math|Rotator|MakeRotator (Math|Float|Lerp 0.0 -35.0 _alpha) (.pitch _returnvalue) (.yaw _returnvalue))))
    (:Finished
      (if (not (== (Math|Float|Lerp 0.0 -35.0 _alpha) 0.0))
        (Development|PrintString "Perdiste")))))

(event Custom|MoveLeft
  (CallFunction|StopMoveLeft))

(event Custom|GameManager
  (switch int (Math|Random|RandomIntegerinRange 0 4)
    (:0
      (CallFunction|UpEvent))
    (:1
      (CallFunction|DownEvent))
    (:2
      (CallFunction|LeftEvent))
    (:3
      (CallFunction|RightEvent))))

(event Custom|DownEvent
  (bind _player_controller (Variables|Default|GetPlayer%20Controller))
  (bind _wb_camionero (Variables|/Game/ElChambas/Blueprints/PlayerControllers/PC_Chambas.PC_Chambas_C|GetWB_Camionero _player_controller))
  (Utilities|FlowControl|DoOnce false
    (:Completed
      (Variables|Default|SetIsDownEvent true)
      (Utilities|FlowControl|Sequence
        (:then_0
          (bind _alpha (Timeline|FrenaEvent Play)
            (:Update
              (Variables|/Script/Engine.SpringArmComponent|SetTargetArmLength (Variables|Default|GetSpringArm) (Math|Float|Lerp (Variables|Default|GetStart%20Target%20Arm%20Length) 3e+02 _alpha)))
            (:Finished
              (if (Variables|Default|GetIsDownEvent)
                (if (Variables|Default|GetbSeAgarro)
                  (CallFunction|Reverse)
                  (else
                    (Development|PrintString "Perdiste")))
                (else
                  (CallFunction|ResetDownEvent))))))
        (:then_1
          (Utilities|FlowControl|Delay 1.0)
          (Default|ShowHideKey _wb_camionero true (Variables|/Game/ElChambas/UI/Widgets/WB_Camionero.WB_Camionero_C|GetDown _wb_camionero))
          (Default|SetWarningText _wb_camionero "Agarrate!" true))))))

(event Custom|LeftEvent
  (bind _returnvalue (Transformation|GetActorRotation))
  (bind _player_controller (Variables|Default|GetPlayer%20Controller))
  (bind _wb_camionero (Variables|/Game/ElChambas/Blueprints/PlayerControllers/PC_Chambas.PC_Chambas_C|GetWB_Camionero _player_controller))
  (Default|ShowHideKey _wb_camionero true (Variables|/Game/ElChambas/UI/Widgets/WB_Camionero.WB_Camionero_C|GetLeft _wb_camionero))
  (Default|SetWarningText _wb_camionero "Te Caes!" true)
  (bind _alpha (Timeline|Timeline_1 Play)
    (:Update
      (Transformation|SetActorRelativeRotation (Math|Rotator|MakeRotator (Math|Float|Lerp 0.0 -35.0 _alpha) (.pitch _returnvalue) (.yaw _returnvalue))))
    (:Finished
      (if (not (== (Math|Float|Lerp 0.0 -35.0 _alpha) 0.0))
        (Development|PrintString "Perdiste")))))

(event Custom|RightEvent
  (bind _returnvalue (Transformation|GetActorRotation))
  (bind _player_controller (Variables|Default|GetPlayer%20Controller))
  (bind _wb_camionero (Variables|/Game/ElChambas/Blueprints/PlayerControllers/PC_Chambas.PC_Chambas_C|GetWB_Camionero _player_controller))
  (Default|ShowHideKey _wb_camionero true (Variables|/Game/ElChambas/UI/Widgets/WB_Camionero.WB_Camionero_C|GetRight _wb_camionero))
  (Default|SetWarningText _wb_camionero "Te caes!" true)
  (bind _alpha (Timeline|Timeline Play)
    (:Update
      (Transformation|SetActorRelativeRotation (Math|Rotator|MakeRotator (Math|Float|Lerp 0.0 35.0 _alpha) (.pitch _returnvalue) (.yaw _returnvalue))))
    (:Finished
      (if (not (== (Math|Float|Lerp 0.0 35.0 _alpha) 0.0))
        (Development|PrintString "Perdiste")))))

(event EventBeginPlay
  (bind _player_controller (Class|INTPlayerControllers|GetPCChambas(Message) (Game|GetPlayerController 0)))
  (bind _output_get (Variables|Default|SetPlayer%20Controller _player_controller))
  (Default|ShowHideWidget _output_get true "NewEnumerator1")
  (Variables|Default|SetStart%20Target%20Arm%20Length (Variables|/Script/Engine.SpringArmComponent|GetTargetArmLength (Variables|Default|GetSpringArm)))
  (bind _returnvalue (Utilities|Time|SetTimerbyEvent (delegate Custom|GameManager) 3.0 true 0.0 1.0))
  (Variables|Default|SetGameManagerTimerHandle _returnvalue))

(fn ConstructionScript)

(fn GetCamioneroZD
  (return self))
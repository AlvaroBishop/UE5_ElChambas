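; BP_MousePawn is a pawn that lets the player pick physics objects with the mouse cursor.
; Space toggles both the cursor and grab mode.
; In that mode, left click traces under the cursor on Visibility, stores and debug-prints any Movable component hit, and grabs it with a PhysicsHandle if it simulates physics.
; Release is an empty stub, and nothing here moves the handle target or lets go.
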(event Input|MouseEvents|LeftMouseButton
  (params (Key :type Key%20Structure :default "None"))
  (bind _returnvalue (Game|GetPlayerController 0))
  (bind _bisgrabmode (Variables|Default|GetbIsGrabMode))
  (bind _hitresult (Game|Player|GetHitResultUnderCursorbyChannel _returnvalue "TraceTypeQuery1" true))
  (bind (_bblockinghit _binitialoverlap _time _distance _location _impactpoint _normal _impactnormal _physmat _hitactor _hitcomponent) (Collision|BreakHitResult _hitresult))
  (bind _mobility (Variables|/Script/Engine.SceneComponent|GetMobility _hitcomponent))
  (:Pressed
    (if _bisgrabmode
      (if (and _bblockinghit (Utilities|Enum|Equal(Enum) _mobility "Movable"))
        (Development|PrintString (Utilities|String|EnumtoString _mobility))
        (bind _output_get (Variables|Default|SetGrabbedComponent _hitcomponent))
        (Development|PrintString (Utilities|GetDisplayName _output_get))
        (if (Physics|IsSimulatingPhysics _output_get "None")
          (Class|PhysicsHandleComponent|GrabComponentatLocation (Variables|Default|GetPhysicsHandle) (Variables|Default|GetGrabbedComponent) "None" (.Location (Collision|BreakHitResult _hitresult)))))))
  (:Released
    (if _bisgrabmode
      _)))

(event Input|KeyboardEvents|SpaceBar
  (params (Key :type Key%20Structure :default "None"))
  (bind _returnvalue (Game|GetPlayerController 0))
  (:Pressed
    (Variables|/Script/Engine.PlayerController|SetbShowMouseCursor _returnvalue (not (Variables|/Script/Engine.PlayerController|GetbShowMouseCursor _returnvalue)))
    (Variables|Default|SetbIsGrabMode (not (Variables|Default|GetbIsGrabMode)))))

(fn ConstructionScript)